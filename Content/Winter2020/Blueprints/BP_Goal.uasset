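; BP_Goal is a goal area actor that tracks how many actors tagged Grayman are inside it.
; At BeginPlay it scales the SMGoal mesh in X and Y by Radius.
; Actor overlap begin and end raise or lower GoalCount for tagged actors, then call AtGoal or LeaveGoal to signal the change.
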(event `self.ReceiveBeginPlay`
  (bind _radius (`self.Radius`))
  (`SceneComponent.SetWorldScale3D` (`self.SM_Goal`) (`KismetMathLibrary.MakeVector` _radius _radius 1.0)))

(event `self.ReceiveActorBeginOverlap`
  (params (OtherActor :type "Actor Object Reference"))
  (if (`self.ActorHasTag` OtherActor "Grayman")
    (`/Engine/EditorBlueprintResources/StandardMacros.IncrementInt` (`self.GoalCount`)
      (:`  `
        (`self.EventAtGoal`)))))

(event `self.ReceiveActorEndOverlap`
  (params (OtherActor :type "Actor Object Reference"))
  (if (`self.ActorHasTag` OtherActor "Grayman")
    (`/Engine/EditorBlueprintResources/StandardMacros.DecrementInt` (`self.GoalCount`)
      (:`  `
        (`self.EventLeaveGoal`)))))

(fn `UserConstructionScript`)