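; Stage manager that runs a level's win and lose rules, HUD and stage progression.
; BeginPlay counts tagged Graymen and weapons and binds goal and pickup events to counters that Tick displays and checks.
; Every Grayman at a goal plus every weapon taken clears the stage, advancing through DT_StageList via the GameInstance index.
; Otherwise, any death of the player or other Graymen shows a failure widget and reloads the level.
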(event `self.ReceiveBeginPlay`
  (`self.CountGrayman`)
  (`self.CountStages`)
  (`self.PrepareWeapons`)
  (`self.InitWidget`)
  (`self.InitObject`))

(event `self.ReceiveEndPlay`
  (params (EndPlayReason :type "EEndPlayReason Enum" :default "Destroyed"))
  (`WidgetLayoutLibrary.RemoveAllWidgets`))

(event `self.ReceiveTick`
  (params (DeltaSeconds :type "Float (single-precision)"))
  (`self.UpdateHud`)
  (bind _cleared (`self.IsStageClear`))
  (if _cleared
    (`/Engine/EditorBlueprintResources/StandardMacros.DoOnce` false
      (:`Completed`
        (bind _returnvalue (`|CreateWidget` "/Game/Winter2020/UI/UI_CLEAR.UI_CLEAR_C"))
        (`UserWidget.AddToViewport` _returnvalue 0)
        (`KismetSystemLibrary.Delay` 2.0)
        (`self.ToNextStage`)))
    (else
      (bind _gameover (`self.IsGameOver`))
      (if _gameover
        (`/Engine/EditorBlueprintResources/StandardMacros.DoOnce` false
          (:`Completed`
            (bind _returnvalue_2 (`|CreateWidget` "/Game/Winter2020/UI/UI_Failed.UI_Failed_C"))
            (`UserWidget.AddToViewport` _returnvalue_2 0)
            (`KismetSystemLibrary.Delay` 2.0)
            (bind _returnvalue_3 (`GameplayStatics.GetCurrentLevelName` true))
            (`GameplayStatics.OpenLevel` (`KismetStringLibrary.Conv_StringToName` _returnvalue_3))))))))

(fn `AtGoal`
  (`/Engine/EditorBlueprintResources/StandardMacros.IncrementInt` (`self.CountGoals`)))

(fn `CountGrayman`
  (bind _outactors (`GameplayStatics.GetAllActorsWithTag` "Grayman"))
  (set `self.NumGoalTargets` (`KismetArrayLibrary.Array_Length` _outactors)))

(fn `CountStages`
  (bind _outrownames (`DataTableFunctionLibrary.GetDataTableRowNames` "/Game/Winter2020/Blueprints/DT_StageList.DT_StageList"))
  (set `self.NumStages` (`KismetArrayLibrary.Array_Length` _outrownames)))

(fn `InitObject`
  (bind _outactors (`GameplayStatics.GetAllActorsOfClass` "/Game/Winter2020/Blueprints/BP_Goal.BP_Goal_C"))
  (for _array_element _outactors
    (add `/Game/Winter2020/Blueprints/BP_Goal.EventAtGoal` _array_element (`|CreateDelegate` :!event `AtGoal`))
    (add `/Game/Winter2020/Blueprints/BP_Goal.EventLeaveGoal` _array_element (`|CreateDelegate` :!event `LeaveGoal`)))
  ;[1 1 1] プレイヤーと他のグレイマンを取得
  (bind _outactors_2 (`GameplayStatics.GetAllActorsOfClass` "/Game/Winter2020/Blueprints/BP_Other.BP_Other_C"))
  (set `self.Others` _outactors_2)
  (bind _returnvalue (`GameplayStatics.GetActorOfClass` "/Game/Winter2020/Blueprints/BP_Player.BP_Player_C"))
  (set `self.Player` _returnvalue))

(fn `InitWidget`
  (bind _returnvalue (`|CreateWidget` "/Game/Winter2020/UI/UI_Hud.UI_Hud_C"))
  (bind _output_get (set `self.UIHud` _returnvalue))
  (`UserWidget.AddToViewport` _output_get 0)
  (`self.UpdateHud`))

(fn `IsGameOver`
  (returns (GameOver :type Boolean))
  (locals (Alive :type Integer))
  (set `local.Alive` (`self.NumGoalTargets`))
  (for _array_element (`self.Others`)
    (bind _killed (`/Game/Winter2020/Blueprints/BP_Other.IsDeath` _array_element))
    (if _killed
      (`/Engine/EditorBlueprintResources/StandardMacros.DecrementInt` (`local.Alive`))))
  (bind _killed_2 (`/Game/Winter2020/Blueprints/BP_Player.IsDeath` (`self.Player`)))
  (if _killed_2
    (`/Engine/EditorBlueprintResources/StandardMacros.DecrementInt` (`local.Alive`)
      (:`  `
        _)))
  (return (!= (`local.Alive`) (`self.NumGoalTargets`))))

(fn `IsStageClear`
  (returns (Cleared :type Boolean))
  (return (and (== (`self.NumGoalTargets`) (`self.CountGoals`)) (== (`self.NumWeapons`) (`self.CountWeapons`)))))

(fn `LeaveGoal`
  (`/Engine/EditorBlueprintResources/StandardMacros.DecrementInt` (`self.CountGoals`)))

(fn `PrepareWeapons`
  (bind _outactors (`GameplayStatics.GetAllActorsWithTag` "Weapon"))
  (bind _output_get (set `self.NumWeapons` (`KismetArrayLibrary.Array_Length` _outactors)))
  (if (> _output_get 0)
    (for _array_element _outactors
      (bind _asbp_weapon (cast `/Game/Winter2020/Blueprints/BP_Weapon` _array_element))
      (add `/Game/Winter2020/Blueprints/BP_Weapon.EventTakeWeapon` _asbp_weapon (`|CreateDelegate` :!event `TakeWeapon`)))))

(fn `TakeWeapon`
  (`/Engine/EditorBlueprintResources/StandardMacros.IncrementInt` (`self.CountWeapons`)))

(fn `ToNextStage`
  (locals (NextStageIndex :type Integer))
  (bind _asbp_game_instance (cast `/Game/Winter2020/Blueprints/BP_GameInstance` (`GameplayStatics.GetGameInstance`)))
  (bind _outrownames (`DataTableFunctionLibrary.GetDataTableRowNames` "/Game/Winter2020/Blueprints/DT_StageList.DT_StageList"))
  (bind _currentstageindex (`/Game/Winter2020/Blueprints/BP_GameInstance.CurrentStageIndex` _asbp_game_instance))
  (set `local.NextStageIndex` (+ _currentstageindex 1))
  (bind _returnvalue (`|GetDataTableRow` "/Game/Winter2020/Blueprints/DT_StageList.DT_StageList" (`|GetArrayItem` _outrownames _currentstageindex))
    (:`then`
      (bind _asbp_game_instance_2 (cast `/Game/Winter2020/Blueprints/BP_GameInstance` (`GameplayStatics.GetGameInstance`)))
      (set `/Game/Winter2020/Blueprints/BP_GameInstance.CurrentStageIndex` (`local.NextStageIndex`) _asbp_game_instance_2)
      (`GameplayStatics.OpenLevel` (`.StageName_2_CFB22F2F4D8C9EB0A34C33B0734B9E93` (break `/Game/Winter2020/Blueprints/ST_Stage` _returnvalue))))
    (:`RowNotFound`
      (`KismetSystemLibrary.PrintString` "End"))))

(fn `UpdateHud`
  (bind _numweapons (`self.NumWeapons`))
  (set `/Game/Winter2020/UI/UI_Hud.GoalCountText` (`|FormatText` "{0}/{1}人" (`self.CountGoals`) (`self.NumGoalTargets`)) (`self.UIHud`))
  (bind _asbp_game_instance (cast `/Game/Winter2020/Blueprints/BP_GameInstance` (`GameplayStatics.GetGameInstance`)))
  (set `/Game/Winter2020/UI/UI_Hud.StageCountText` (`|FormatText` "{0}/{1}" (`/Game/Winter2020/Blueprints/BP_GameInstance.CurrentStageIndex` _asbp_game_instance) (`self.NumStages`)) (`self.UIHud`))
  (if (> _numweapons 0)
    (set `/Game/Winter2020/UI/UI_Hud.WeaponCountText` (`|FormatText` "{0}/{1}個" (`self.CountWeapons`) _numweapons) (`self.UIHud`))
    (else
      (set `/Game/Winter2020/UI/UI_Hud.WeaponCountText` "-/-個" (`self.UIHud`)))))

(fn `UserConstructionScript`)