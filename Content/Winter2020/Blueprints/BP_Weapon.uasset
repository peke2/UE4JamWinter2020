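; BP_Weapon is a spinning weapon pickup that an overlapping actor can take once.
; On overlap it queries the other actor through message calls and, if that actor has no weapon, tells it to take one.
; The pickup then plays the PistolRaise timeline, fires the TakeWeapon event, and destroys itself after a short delay.
; Tick rotates it slowly while idle and faster once Fading is set.
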(event `self.ReceiveActorBeginOverlap`
  (params (OtherActor :type "Actor Object Reference"))
  (bind _has (message `/Game/Winter2020/Blueprints/IF_Grayman.HasWeapon` OtherActor))
  (if (not _has)
    (`/Engine/EditorBlueprintResources/StandardMacros.DoOnce` false
      (:`Completed`
        (message `/Game/Winter2020/Blueprints/IF_Grayman.TakeWeapon` OtherActor)
        (`AudioComponent.Play` (`self.Pistol_Raise`) 0.0)
        (`self.EventTakeWeapon`)
        (set `self.Fading` true)
        (`KismetSystemLibrary.Delay` 1.0)
        (`self.K2_DestroyActor`)))))

(event `self.ReceiveTick`
  (params (DeltaSeconds :type "Float (single-precision)"))
  (if (`self.Fading`)
    (`self.K2_AddActorLocalRotation` (struct :`Yaw` 12.0))
    (else
      (`self.K2_AddActorLocalRotation` (struct :`Yaw` 1.0)))))

(fn `UserConstructionScript`)